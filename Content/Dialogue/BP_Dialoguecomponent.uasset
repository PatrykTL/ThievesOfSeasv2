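; Dialogue component that runs branching conversations with a named speaker, showing lines and choices in WB_Dialogue.
; Each Interact shows the current DataTable row and stores the next row, table and end flag it points to, closing the widget after a final line.
; Open-ended rows spawn WB_Options buttons, whose OptionSelected callback follows the chosen row and calls StartQuest on TreasureIslandGameMode.
; Input switches to Game and UI with a visible cursor during dialogue.
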(event Custom|Option%20Selected
  (params (RowName :type Name) (DataTable :type Data%20Table%20Object%20Reference) (QuestName :type Name))
  (Widget|Panel|ClearChildren (Variables|/Game/Dialogue/WB_Dialogue.WB_Dialogue_C|GetOptionsScrollBox (Variables|Default|GetDialogueWidget)))
  (bind _returnvalue (Utilities|GetDataTableRow DataTable RowName)
    (:then
      (Default|UpdateDialogue (Variables|Default|GetDialogueWidget) (.Dialogue (Utilities|Struct|BreakDialogue_Structure _returnvalue)))
      (Variables|Default|SetRowName (.Row (Utilities|Struct|BreakDialogue_Structure _returnvalue)))
      (Variables|Default|SetEndDialogue (.EndDialogue? (Utilities|Struct|BreakDialogue_Structure _returnvalue)))
      (Variables|Default|SetDataTable (.Datatable (Utilities|Struct|BreakDialogue_Structure _returnvalue)))
      (bind _astreasure_island_game_mode (Utilities|Casting|CastToTreasureIslandGameMode (Game|GetGameMode)))
      (Default|StartQuest _astreasure_island_game_mode QuestName))))

(event EventLeaveDialogue
  (Utilities|IsValid (Variables|Default|GetDialogueWidget)
    (:Is%20Valid
      (CallFunction|RemoveDialogue)
      (CallFunction|UnlockCameraandHideMouse))))

(event EventInteract
  (params (playerref :type Player%20Object%20Reference))
  (if (Variables|Default|GetEndDialogue)
    (CallFunction|RemoveDialogue)
    (CallFunction|UnlockCameraandHideMouse)
    (else
      (Utilities|IsValid (Variables|Default|GetDialogueWidget)
        (:Is%20Valid
          (bind (_openendeddialogue_ _openendeddialogueoptions) (CallFunction|UpdateDialogue))
          (CallFunction|LockCameraandShowMouse)
          (CallFunction|CreateOptionsButtons _openendeddialogue_ _openendeddialogueoptions))
        (:Is%20Not%20Valid
          (bind (_openendeddialogue__2 _openendeddialogueoptions_2) (CallFunction|CreateDialogueWidget (Variables|Default|GetRowName)))
          (CallFunction|LockCameraandShowMouse)
          (CallFunction|CreateOptionsButtons _openendeddialogue__2 _openendeddialogueoptions_2))))))

(fn RemoveDialogue
  (Widget|RemovefromParent (Variables|Default|GetDialogueWidget))
  (Variables|Default|SetEndDialogue false)
  (Variables|Default|SetDialogueWidget 0))

(fn UpdateDialogue
  (bind _returnvalue (Utilities|GetDataTableRow (Variables|Default|GetDataTable) (Variables|Default|GetRowName))
    (:then
      (Default|UpdateDialogue (Variables|Default|GetDialogueWidget) (.Dialogue (Utilities|Struct|BreakDialogue_Structure _returnvalue)))
      (Variables|Default|SetRowName (.Row (Utilities|Struct|BreakDialogue_Structure _returnvalue)))
      (Variables|Default|SetDataTable (.Datatable (Utilities|Struct|BreakDialogue_Structure _returnvalue)))
      (Variables|Default|SetEndDialogue (.EndDialogue? (Utilities|Struct|BreakDialogue_Structure _returnvalue)))
      (return (.OpenEndedDialogue? (Utilities|Struct|BreakDialogue_Structure _returnvalue)) (.OpenEndedDialogueOptions (Utilities|Struct|BreakDialogue_Structure _returnvalue))))))

(fn CreateDialogueWidget
  (params (RowName :type Name))
  (bind _returnvalue (Utilities|GetDataTableRow (Variables|Default|GetDataTable) RowName)
    (:then
      (bind _returnvalue_2 (UserInterface|CreateWidget "/Game/Dialogue/WB_Dialogue.WB_Dialogue_C" 0 (Utilities|Text|ToText(Name) (Variables|Default|GetName)) (.Dialogue (Utilities|Struct|BreakDialogue_Structure _returnvalue))))
      (bind _output_get (Variables|Default|SetDialogueWidget _returnvalue_2))
      (UserInterface|Viewport|AddtoViewport _output_get 0)
      (Variables|Default|SetRowName (.Row (Utilities|Struct|BreakDialogue_Structure _returnvalue)))
      (Variables|Default|SetDataTable (.Datatable (Utilities|Struct|BreakDialogue_Structure _returnvalue)))
      (Variables|Default|SetEndDialogue (.EndDialogue? (Utilities|Struct|BreakDialogue_Structure _returnvalue))))
    (:RowNotFound
      _))
  (return (.OpenEndedDialogue? (Utilities|Struct|BreakDialogue_Structure _returnvalue)) (.OpenEndedDialogueOptions (Utilities|Struct|BreakDialogue_Structure _returnvalue))))

(fn CreateOptionsButtons
  (params (Condition :type Boolean) (Array :type Array%20of%20Options%20Dialogue%20Structure%20Structures))
  (if Condition
    (for _array_element Array
      (bind _returnvalue (UserInterface|CreateWidget "/Game/Dialogue/WB_Options.WB_Options_C" 0 (Utilities|Text|ToText(Name) (.OptionName (Utilities|Struct|BreakOptionsDialogue_Structure _array_element))) self (.Row (Utilities|Struct|BreakOptionsDialogue_Structure _array_element)) (.Datatable (Utilities|Struct|BreakOptionsDialogue_Structure _array_element)) (.StartedQuestName (Utilities|Struct|BreakOptionsDialogue_Structure _array_element))))
      (Widget|Panel|AddChild (Variables|/Game/Dialogue/WB_Dialogue.WB_Dialogue_C|GetOptionsScrollBox (Variables|Default|GetDialogueWidget)) _returnvalue))))

(fn LockCameraandShowMouse
  (bind _returnvalue (Game|GetPlayerController 0))
  (Input|SetInputModeGameandUI _returnvalue 0 "LockAlways" true false)
  (Variables|/Script/Engine.PlayerController|SetbShowMouseCursor _returnvalue true))

(fn UnlockCameraandHideMouse
  (bind _returnvalue (Game|GetPlayerController 0))
  (Input|SetInputModeGameOnly _returnvalue true)
  (Variables|/Script/Engine.PlayerController|SetbShowMouseCursor _returnvalue false))